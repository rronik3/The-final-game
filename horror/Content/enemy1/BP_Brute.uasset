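; BP_Brute is an enemy character with health, random hit reactions and a ragdoll death.
; It links itself to its HealthWidget_Enemy, which shows while BP_Girl overlaps its Sphere and hides when she leaves.
; AnyDamage plays one of two hit montages and subtracts Health.
; At zero it starts a death montage, picked by a 0–19 roll over two options, then switches to physics after a short delay.
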(event `self.ReceiveBeginPlay`
  ; Подключение виджета
  (bind _ashealth_widget_enemy (cast `/Game/enemy1/HealthWidget_Enemy` (`WidgetComponent.GetUserWidgetObject` (`self.HealthWidget`))))
  (set `/Game/enemy1/HealthWidget_Enemy.BP_Brute` self _ashealth_widget_enemy))

(event `self.ReceiveAnyDamage`
  (params (Damage :type "Float (single-precision)") (DamageType :type "DamageType Object Reference") (InstigatedBy :type "Controller Object Reference") (DamageCauser :type "Actor Object Reference"))
  (bind _mesh (`self.Mesh`))
  ; Damage
  (`|PlayMontage` (`self.Mesh`) (select `int` (`KismetMathLibrary.RandomInteger` 2) :`0` (`self.HitReact1`) :`1` (`self.HitReact2`))
    (:`then`
      (set `self.Health` (- (`self.Health`) Damage))
      (if (<= (`self.Health`) 0.0)
        ; Death
        (`PrimitiveComponent.SetCollisionEnabled` _mesh "QueryAndPhysics")
        (`self.PlayAnimMontage` (select `int` (`KismetMathLibrary.RandomInteger` 20) :`0` (`self.Death1`) :`1` (`self.Death2`)))
        (`KismetSystemLibrary.Delay` 0.5)
        (`PrimitiveComponent.SetSimulatePhysics` _mesh true)
        (`PrimitiveComponent.SetCollisionEnabled` (`self.CapsuleComponent`) "NoCollision")
        (`PrimitiveComponent.SetCollisionEnabled` (`self.Mesh`) "PhysicsOnly")))))

(event `self.Sphere.OnComponentBeginOverlap`
  (params (OverlappedComponent :type "PrimitiveComponent Object Reference") (OtherActor :type "Actor Object Reference") (OtherComp :type "PrimitiveComponent Object Reference") (OtherBodyIndex :type Integer) (bFromSweep :type Boolean) (SweepResult :type "HitResult Structure (by ref)"))
  (cast `/Game/MainCharacter/BP_Girl` OtherActor)
  (`SceneComponent.SetVisibility` (`self.HealthWidget`) true false))

(event `self.Sphere.OnComponentEndOverlap`
  (params (OverlappedComponent :type "PrimitiveComponent Object Reference") (OtherActor :type "Actor Object Reference") (OtherComp :type "PrimitiveComponent Object Reference") (OtherBodyIndex :type Integer))
  (cast `/Game/MainCharacter/BP_Girl` OtherActor)
  (`SceneComponent.SetVisibility` (`self.HealthWidget`) false false))

(fn `UserConstructionScript`)