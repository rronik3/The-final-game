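; BP_Horse is a rideable horse character with mouse look, directional movement and a Shift sprint that changes walk speed.
; While BP_Girl overlaps the Box, the horse binds its HorseRide event to her HorseRide dispatcher, unbinding on exit.
; Mounting stores the player character, possesses the horse and shows a SkeletalMesh component.
; Pressing E moves the rider to DeattachCharacter, repossesses them and hides that mesh.
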(event `InputAxis|LookUpDown`
  (params (AxisValue :type "Float (single-precision)"))
  ; Mouse
  (`self.AddControllerPitchInput` AxisValue))

(event `Key|LeftShift`
  (params (Key :type "Key Structure"))
  (:`Pressed`
    (set `self.isSprint` true))
  (:`Released`
    (set `self.isSprint` false)))

(event `InputAxis|LookLeftRight`
  (params (AxisValue :type "Float (single-precision)"))
  ; Mouse
  (`self.AddControllerYawInput` AxisValue))

(event `InputAxis|MoveForwardBack`
  (params (AxisValue :type "Float (single-precision)"))
  ; Ходьба
  (`self.AddMovementInput` (`SceneComponent.GetForwardVector` (`self.CapsuleComponent`)) AxisValue)
  ; Sprint
  (set `CharacterMovementComponent.MaxWalkSpeed` 300.0 (`self.CharacterMovement`))
  (if (`self.isSprint`)
    (set `CharacterMovementComponent.MaxWalkSpeed` 600.0 (`self.CharacterMovement`))))

(event `InputAxis|MoveRightLeft`
  (params (AxisValue :type "Float (single-precision)"))
  ; Ходьба
  (`self.AddMovementInput` (`SceneComponent.GetRightVector` (`self.CapsuleComponent`)) AxisValue)
  ; Sprint
  (set `CharacterMovementComponent.MaxWalkSpeed` 300.0 (`self.CharacterMovement`))
  (if (`self.isSprint`)
    (set `CharacterMovementComponent.MaxWalkSpeed` 600.0 (`self.CharacterMovement`))))

(event `self.Box.OnComponentBeginOverlap`
  (params (OverlappedComponent :type "PrimitiveComponent Object Reference") (OtherActor :type "Actor Object Reference") (OtherComp :type "PrimitiveComponent Object Reference") (OtherBodyIndex :type Integer) (bFromSweep :type Boolean) (SweepResult :type "HitResult Structure (by ref)"))
  ; сесть на лошадь в BoxCollision
  (bind _asbp_girl (cast `/Game/MainCharacter/BP_Girl` OtherActor))
  (add `/Game/MainCharacter/BP_Girl.HorseRide` _asbp_girl (delegate `HorseRide`)))

(event `HorseRide`
  ; сесть на лошадь в BoxCollision
  (set `self.HorseMan` (`GameplayStatics.GetPlayerCharacter` 0))
  (`Controller.Possess` (`GameplayStatics.GetPlayerController` 0) self)
  (`SceneComponent.SetVisibility` (`self.SkeletalMesh`) true false))

(event `self.Box.OnComponentEndOverlap`
  (params (OverlappedComponent :type "PrimitiveComponent Object Reference") (OtherActor :type "Actor Object Reference") (OtherComp :type "PrimitiveComponent Object Reference") (OtherBodyIndex :type Integer))
  ; запрет сесть
  (bind _asbp_girl (cast `/Game/MainCharacter/BP_Girl` OtherActor))
  (clear `/Game/MainCharacter/BP_Girl.HorseRide` _asbp_girl))

(event `Key|E`
  (params (Key :type "Key Structure"))
  (bind _horseman (`self.HorseMan`))
  ; Слезть
  (:`Pressed`
    (`self.K2_SetActorTransform` _horseman (`KismetMathLibrary.MakeTransform` (`SceneComponent.K2_GetComponentLocation` (`self.DeattachCharacter`)) (struct) (`SceneComponent.K2_GetComponentScale` (`Actor.RootComponent` _horseman))) false false)
    (`Controller.Possess` (`GameplayStatics.GetPlayerController` 0) (`self.HorseMan`))
    (`SceneComponent.SetVisibility` (`self.SkeletalMesh`) false false)))

(fn `UserConstructionScript`)